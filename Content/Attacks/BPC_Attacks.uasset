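; Attack component that gives its owning actor a hitscan bullet attack and a magic projectile spell.
; FireBullets line-traces for pawns and damages the first hit on another team, while MagicSpell spawns one of two targeted energy projectiles.
; Projectile impacts deal damage without a team check and fire OnAttackEnded; both attacks report damage events.
; A damage-all helper hits each non-team actor once but is not called in these graphs.
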(event Custom|Magic%20Spell
  (params (SpawnTransform :type Transform) (Target :type Actor%20Object%20Reference) (DamageInfo :type S%20Damage%20Info%20Structure) (Alt :type Boolean))
  (bind _returnvalue (Game|SpawnActorfromClass (select Alt "/Game/Projectiles/BP_Projectile_GreenEnergy.BP_Projectile_GreenEnergy_C" "/Game/Projectiles/BP_Projectile_BlueEnergy.BP_Projectile_BlueEnergy_C") SpawnTransform "Undefined" "MultiplyWithRoot" (Components|GetOwner) 1e+03 0.0 Target false 0))
  (EventDispatchers|AssignOnProjectileImpact _returnvalue (delegate Custom|OnProjectileHit))
  (Collision|IgnoreActorwhenMoving (Actor|GetComponentbyClass (Components|GetOwner) "/Script/Engine.CapsuleComponent") _returnvalue true))

(event Custom|Fire%20Bullets
  (params (StartTrace :type Vector) (EndTrace :type Vector) (DamageInfo :type S%20Damage%20Info%20Structure))
  (bind (_outhits _returnvalue) (Class|KismetSystemLibrary|LineTraceMultiforObjects StartTrace EndTrace (Utilities|Array|MakeArray "ObjectTypeQuery3") false (Utilities|Array|MakeArray (Components|GetOwner)) "ForDuration" true))
  (if _returnvalue
    (bind _actordamaged (CallFunction|DamageFirstNonTeamMembers _outhits DamageInfo))
    (Class|AISenseDamage|ReportDamageEvent _actordamaged (Components|GetOwner) (.Amount (Utilities|Struct|BreakS_DamageInfo DamageInfo)) (Transformation|GetActorLocation (Components|GetOwner)) "0, 0, 0" "None")))

(event Custom|OnProjectileHit
  (params (OtherActor :type Actor%20Object%20Reference) (Hit :type Hit%20Result%20Structure))
  (bind _returnvalue (Components|GetOwner))
  (Class|BPIDamageable|TakeDamage(Message) OtherActor (stale Custom|Magic%20Spell DamageInfo) _returnvalue)
  (Class|AISenseDamage|ReportDamageEvent 0 _returnvalue (.Amount (Utilities|Struct|BreakS_DamageInfo (stale Custom|Magic%20Spell DamageInfo))) (Transformation|GetActorLocation (Components|GetOwner)) "0, 0, 0" "None")
  (Default|CallOnAttackEnded))

(fn DamageAllNonTeamMembers
  (params (Hits :type Array%20of%20Hit%20Result%20Structures) (DamageInfo :type S%20Damage%20Info%20Structure))
  (for _array_element Hits
    (bind _teamnumber (Class|BPIDamageable|GetTeamNumber(Message) (.HitActor (Collision|BreakHitResult _array_element))))
    (bind _teamnumber_2 (Class|BPIDamageable|GetTeamNumber(Message) (Components|GetOwner)))
    (if (and (!= _teamnumber_2 _teamnumber) (not (Utilities|Array|ContainsItem (LocalVariables|GetActorsDamagedSoFar) (.HitActor (Collision|BreakHitResult _array_element)))))
      (Class|BPIDamageable|TakeDamage(Message) (.HitActor (Collision|BreakHitResult _array_element)) DamageInfo (Components|GetOwner))
      (Utilities|Array|AddUnique (LocalVariables|GetActorsDamagedSoFar) (.HitActor (Collision|BreakHitResult _array_element)))))
  (return (LocalVariables|GetActorsDamagedSoFar)))

(fn DamageFirstNonTeamMembers
  (params (Hits :type Array%20of%20Hit%20Result%20Structures) (DamageInfo :type S%20Damage%20Info%20Structure))
  (bind _array_element (Utilities|Array|ForEachLoopwithBreak Hits :!label _label)
    (:LoopBody
      (bind _teamnumber (Class|BPIDamageable|GetTeamNumber(Message) (.HitActor (Collision|BreakHitResult _array_element))))
      (bind _teamnumber_2 (Class|BPIDamageable|GetTeamNumber(Message) (Components|GetOwner)))
      (if (!= _teamnumber_2 _teamnumber)
        (Class|BPIDamageable|TakeDamage(Message) (.HitActor (Collision|BreakHitResult _array_element)) DamageInfo (Components|GetOwner))
        (Utilities|FlowControl|Sequence
          (:then_0
            (goto _label Break)))))))