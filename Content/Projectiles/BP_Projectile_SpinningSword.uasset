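; Spinning sword projectile Blueprint that continuously rotates its mesh.
; On BeginPlay, after the parent logic, it starts SwordSpinTimeline, which drives the mesh's world yaw while keeping its current roll and pitch.
; When the timeline finishes, the SpinSword event calls itself to replay from the start, looping the spin indefinitely.
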(event Custom|SpinSword
  (bind _mesh (Variables|Character|GetMesh))
  (bind _returnvalue (Transformation|GetWorldRotation _mesh))
  (bind _zrotate (Timeline|SwordSpinTimeline PlayFromStart)
    (:Update
      (Transformation|SetWorldRotation (Variables|Character|GetMesh) (Math|Rotator|MakeRotator (.roll _returnvalue) (.pitch _returnvalue) _zrotate) false false))
    (:Finished
      (CallFunction|SpinSword))))

(event EventBeginPlay
  (|CallParentFunction)
  (CallFunction|SpinSword))

(event Collision|EventActorBeginOverlap
  (params (OtherActor :type Actor%20Object%20Reference)))

(event EventTick
  (params (DeltaSeconds :type Float%20%28single-precision%29)))

(fn ConstructionScript
  (|CallParentFunction))