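; BP_Enemy_Melee is a sword-wielding enemy that implements attack, equip and unequip actions through montages.
; Attack plays a montage and signals its end whether completed or interrupted.
; Montage notifies time spawning the sword onto a hand socket and destroying it on sheathing, updating the wielding flag.
; Equip and unequip fire their dispatchers only on montage completion, with no interruption handling.
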(event EventBeginPlay)

(event EventEquipWeapon
  (bind _notifyname (Animation|Montage|PlayMontage (Variables|Character|GetMesh) "/Game/Animation/SheathSword/UnSheathing_Sword_Montage.UnSheathing_Sword_Montage")
    (:OnCompleted
      (Default|CallOnWeaponEquipped))
    (:OnNotifyBegin
      (switch name _notifyname
        (:Open%20Sword
          (bind _returnvalue (Game|SpawnActorfromClass "/Game/Weapons/BP_Weapon_Sword.BP_Weapon_Sword_C" (Transformation|GetActorTransform) "Undefined" "MultiplyWithRoot" 0 0))
          (Variables|Default|SetWeaponActor _returnvalue)
          (Transformation|AttachComponentToComponent _returnvalue (Variables|Character|GetMesh) "hand_rSocket Sword" "SnapToTarget" "SnapToTarget" "SnapToTarget" true)
          (Variables|Default|SetisWieldingWeapon true))))))

(event EventUnEquipWeapon
  (bind _notifyname (Animation|Montage|PlayMontage (Variables|Character|GetMesh) "/Game/Animation/SheathSword/Sheathing_Sword_Montage.Sheathing_Sword_Montage")
    (:OnCompleted
      (Default|CallOnWeaponUnEquipped))
    (:OnNotifyBegin
      (switch name _notifyname
        (:Drop%20Sword
          (Actor|DestroyActor (Variables|Default|GetWeaponActor))
          (Variables|Default|SetisWieldingWeapon false))))))

(event Collision|EventActorBeginOverlap
  (params (OtherActor :type Actor%20Object%20Reference)))

(event EventTick
  (params (DeltaSeconds :type Float%20%28single-precision%29)))

(event EventAttack
  (Animation|Montage|PlayMontage (Variables|Character|GetMesh) "/Game/Animation/Attack1_Montage.Attack1_Montage"
    (:OnCompleted
      _)
    (:OnInterrupted
      _))
  (Default|CallOnEventEnd))

(fn ConstructionScript
  (|CallParentFunction))