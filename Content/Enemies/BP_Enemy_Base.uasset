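; Base enemy character Blueprint providing melee attack, sword wield and sheathe actions, patrol route lookup and movement speed presets.
; Montage notifies time the sword's spawn and attachment to the hand socket, and its destruction on sheathing, while tracking the wielding state.
; Event dispatchers report when the attack finishes or is interrupted and when wield or sheathe montages complete.
; SetMovementSpeed maps a speed state to the walk speed limit, from idle to sprint.
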(event Custom|Wield%20Sword
  (bind _notifyname (Animation|Montage|PlayMontage (Variables|Character|GetMesh) "/Game/Animation/UnSheathing_Sword_Montage.UnSheathing_Sword_Montage")
    (:OnCompleted
      (Default|CallOnWieldSword))
    (:OnNotifyBegin
      (switch name _notifyname
        (:Open%20Sword
          (bind _returnvalue (Game|SpawnActorfromClass "/Game/Weapons/BP_Sword.BP_Sword_C" (Transformation|GetActorTransform) "Undefined" "MultiplyWithRoot" 0 0))
          (Variables|Default|SetSword%20Actor _returnvalue)
          (Transformation|AttachComponentToComponent _returnvalue (Variables|Character|GetMesh) "hand_rSocket Sword" "SnapToTarget" "SnapToTarget" "SnapToTarget" true)
          (Variables|Default|SetisWieldingSword true))))))

(event Custom|Attack
  (Animation|Montage|PlayMontage (Variables|Character|GetMesh) "/Game/Animation/Montage_Attack1.Montage_Attack1"
    (:OnCompleted
      _)
    (:OnInterrupted
      _))
  (Default|CallOnEventEnd))

(event Custom|Sheath%20Sword
  (bind _notifyname (Animation|Montage|PlayMontage (Variables|Character|GetMesh) "/Game/Animation/Sheathing_Sword_Montage.Sheathing_Sword_Montage")
    (:OnCompleted
      (Default|CallOnSheathSword))
    (:OnNotifyBegin
      (switch name _notifyname
        (:Drop%20Sword
          (Actor|DestroyActor (Variables|Default|GetSword%20Actor))
          (Variables|Default|SetisWieldingSword false))))))

(event EventBeginPlay)

(fn ConstructionScript)

(fn GetPatrolRoute
  (return (Variables|AI|GetPatrol%20Route)))

(fn SetMovementSpeed
  (params (Speed :type E_MovementSpeed%20Enum :default "NewEnumerator0"))
  (bind _output_get (Variables|/Script/Engine.CharacterMovementComponent|SetMaxWalkSpeed (Variables|Character|GetCharacterMovement) (Utilities|Select :Index Speed :NewEnumerator0 0.0 :NewEnumerator1 1e+02 :NewEnumerator2 3e+02 :NewEnumerator3 5e+02)))
  (return _output_get))